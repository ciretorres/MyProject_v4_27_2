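; BP_EnemyController is an AI controller that patrols its enemy pawn along a looping list of waypoint actors.
; On BeginPlay it caches the possessed ThirdPersonCharacter, whose ArrayTarget holds the waypoints, and starts the first move.
; Tick polls the distance to the current target and, within a fixed radius, advances the index with wraparound and issues MoveToLocation, rather than waiting for move-completed callbacks.
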(event EventBeginPlay
  ;[1 1 1] Save variable enemy
  (bind _asthird_person_character (Utilities|Casting|CastToThirdPersonCharacter (Pawn|GetControlledPawn)))
  (Variables|Default|SetEnemy _asthird_person_character)
  (CallFunction|Move))

(event EventTick
  (params (DeltaSeconds :type Float%20%28single-precision%29))
  (bind _isnear (CallFunction|IsNear))
  (if _isnear
    (CallFunction|Move)))

(fn ConstructionScript)

(fn GetLocationWaypoint
  (bind _output_get (Variables|Default|SetCurrentWaypoint (+ (Variables|Default|GetCurrentWaypoint) 1)))
  (if (> _output_get (Utilities|Array|LastIndex (Variables|/Game/ThirdPersonBP/Blueprints/ThirdPersonCharacter.ThirdPersonCharacter_C|GetArrayTarget (Variables|Default|GetEnemy))))
    (Variables|Default|SetCurrentWaypoint 0))
  (return (Transformation|GetActorLocation (Utilities|Array|Get(acopy) (Variables|/Game/ThirdPersonBP/Blueprints/ThirdPersonCharacter.ThirdPersonCharacter_C|GetArrayTarget (Variables|Default|GetEnemy)) (Variables|Default|GetCurrentWaypoint)))))

(fn IsNear
  (return (< (Math|Vector|VectorLength (- (Transformation|GetActorLocation (Variables|Default|GetEnemy)) (Variables|Default|GetTargetPosition))) 1.5e+02)))

(fn Move
  (bind _returnvalue (CallFunction|GetLocationWaypoint))
  (bind _output_get (Variables|Default|SetTargetPosition _returnvalue))
  (AI|Navigation|MovetoLocation _output_get -1.0 true true false true 0))